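; Level-art tool Blueprint that builds modular stairs from a chosen static mesh as hierarchical instanced meshes in the construction script.
; With ScaleToMatchEnd on, it derives instance counts and scales from mesh bounds and the LastInstanceEnd vector, adjusting step height to fit the rise.
; Otherwise, it places unscaled steps from manual height and width counts.
; Both modes repeat steps across the width and apply length and rotation corrections.
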(event EventBeginPlay)

(event Collision|EventActorBeginOverlap
  (params (OtherActor :type Actor%20Object%20Reference)))

(event EventTick
  (params (DeltaSeconds :type Float%20%28single-precision%29)))

(fn ConstructionScript
  (bind _correctionlengthvalues (Variables|Default|GetCorrectionLengthValues))
  (bind _correctionrotationvalues (Variables|Default|GetCorrectionRotationValues))
  (bind _correctionlengthvalues_2 (Variables|Default|GetCorrectionLengthValues))
  (bind _lastinstanceend (Variables|Default|GetLastInstanceEnd))
  (Utilities|FlowControl|Sequence
    (:then_0
      ;[1 1 1] Let User set the static Mesh
      (CallFunction|InstantiateSingleHierarchicalInstancedStaticMesh (Variables|Default|GetInstanceGroupStairs) (Variables|Default|GetStaticMesh)))
    (:then_1
      (bind (_meshxlength _meshylength _meshzlength) (CallFunction|GetMeshLengths (Variables|Default|GetStaticMesh) (Variables|Default|GetAxisToScaleBy) false false false))
      (bind _output_get (Variables|Default|SetMeshLengthX _meshxlength))
      (bind _output_get_2 (Variables|Default|SetMeshLengthY _meshylength))
      (bind _output_get_3 (Variables|Default|SetMeshLengthZ _meshzlength)))
    (:then_2
      (bind _output_get_4 (Variables|Default|SetDistanceToEndX (.x _lastinstanceend)))
      (bind _output_get_5 (Variables|Default|SetDistanceToEndY (.y _lastinstanceend)))
      (bind _output_get_6 (Variables|Default|SetDistanceToEndZ (.z _lastinstanceend))))
    (:then_3
      (bind (_scaletomatchend _instancecountx _instancecounty _instancecountz) (CallFunction|CalculateInstanceCountsandMeshScales (Math|Vector|MakeVector _output_get_4 _output_get_5 _output_get_6) (Math|Vector|MakeVector _output_get _output_get_2 _output_get_3)))
      (Variables|Default|SetScaleToMatchEndX (.x _scaletomatchend))
      (Variables|Default|SetScaleToMatchEndY (.y _scaletomatchend))
      (Variables|Default|SetScaleToMatchEndZ (.z _scaletomatchend))
      (Variables|Default|SetInstanceCount_X _instancecountx)
      (Variables|Default|SetInstanceCount_Y _instancecounty)
      (Variables|Default|SetInstanceCount_Z _instancecountz))
    (:then_4
      (if (Variables|Default|GetScaleToMatchEnd?)
        ;[1 1 1] Manual Adjustments of the mesh length and the scalar value
        (Variables|Default|SetMeshLengthZ (* (Variables|Default|GetMeshLengthZ) (/ (Variables|Default|GetInstanceCount_Z) (Variables|Default|GetInstanceCount_X))))
        (Variables|Default|SetScaleToMatchEndZ (/ (* (Variables|Default|GetMeshLengthZ) (/ (Variables|Default|GetInstanceCount_Z) (Variables|Default|GetInstanceCount_X))) (Variables|Default|GetMeshLengthZ)))
        (for _index (range 0 (- (Variables|Default|GetInstanceCount_X) 1))
          (Components|InstancedStaticMesh|AddInstance (Variables|Default|GetInstanceGroupStairs) (Math|Transform|MakeTransform (Math|Vector|MakeVector (* (Variables|Default|GetScaleToMatchEndX) (* (+ (Variables|Default|GetMeshLengthX) (.x _correctionlengthvalues_2)) _index)) 0.0 (* (+ (Variables|Default|GetMeshLengthZ) (.z _correctionlengthvalues_2)) _index)) _correctionrotationvalues (Math|Vector|MakeVector (Variables|Default|GetScaleToMatchEndX) (Variables|Default|GetScaleToMatchEndY) (Variables|Default|GetScaleToMatchEndZ))) false)
          (for _index_2 (range 0 (- (Variables|Default|GetInstanceCount_Y) 2))
            (Components|InstancedStaticMesh|AddInstance (Variables|Default|GetInstanceGroupStairs) (Math|Transform|MakeTransform (Math|Vector|MakeVector (* (Variables|Default|GetScaleToMatchEndX) (* (+ (Variables|Default|GetMeshLengthX) (.x _correctionlengthvalues)) _index)) (* (Variables|Default|GetScaleToMatchEndY) (* (+ (Variables|Default|GetMeshLengthY) (.y _correctionlengthvalues)) (+ _index_2 1))) (* (+ (Variables|Default|GetMeshLengthZ) (.z _correctionlengthvalues)) _index)) _correctionrotationvalues (Math|Vector|MakeVector (Variables|Default|GetScaleToMatchEndX) (Variables|Default|GetScaleToMatchEndY) (Variables|Default|GetScaleToMatchEndZ))) false)))
        (else
          (CallFunction|CreateInstancebyManualCount))))))

(fn CreateInstancebyManualCount
  (bind _correctionlengthvalues (Variables|Default|GetCorrectionLengthValues))
  (bind _correctionlengthvalues_2 (Variables|Default|GetCorrectionLengthValues))
  (for _index (range 0 (- (Variables|Default|GetManual_InstanceCountHeight) 1))
    ;[1 1 1] Creating the instances
    (Components|InstancedStaticMesh|AddInstance (Variables|Default|GetInstanceGroupStairs) (Math|Transform|MakeTransform (Math|Vector|MakeVector (* (+ (Variables|Default|GetMeshLengthX) (.x _correctionlengthvalues_2)) _index) 0.0 (* (+ (Variables|Default|GetMeshLengthZ) (.z _correctionlengthvalues_2)) _index)) (Variables|Default|GetCorrectionRotationValues)) false)
    (for _index_2 (range 0 (- (Variables|Default|GetManual_InstanceCountWidth) 2))
      (Components|InstancedStaticMesh|AddInstance (Variables|Default|GetInstanceGroupStairs) (Math|Transform|MakeTransform (Math|Vector|MakeVector (* (+ (Variables|Default|GetMeshLengthX) (.x _correctionlengthvalues)) _index) (* (+ (Variables|Default|GetMeshLengthY) (.y _correctionlengthvalues)) (+ _index_2 1)) (* (+ (Variables|Default|GetMeshLengthZ) (.z _correctionlengthvalues)) _index)) (Variables|Default|GetCorrectionRotationValues)) false))))