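; BP_ModularFloor is a level art tool that tiles a chosen mesh into a floor grid on X and Y using hierarchical instanced static meshes.
; The construction script measures the mesh and the distance to LastInstanceEnd, then derives instance counts and scales.
; With ScaleToMatchEnd on, tiles are scaled to match that end point; otherwise, manual counts place them unscaled.
; Both modes apply spacing and rotation corrections.
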(event EventBeginPlay)

(event Collision|EventActorBeginOverlap
  (params (OtherActor :type Actor%20Object%20Reference)))

(event EventTick
  (params (DeltaSeconds :type Float%20%28single-precision%29)))

(fn ConstructionScript
  (bind _correctionlength (Variables|Default|GetCorrectionLength))
  (Utilities|FlowControl|Sequence
    (:then_0
      ;[1 1 1] Allowing the user to set the mesh
      (CallFunction|InstantiateSingleHierarchicalInstancedStaticMesh (Variables|Default|GetInstanceGroupFloor) (Variables|Default|GetStaticMesh)))
    (:then_1
      (bind (_meshxlength _meshylength _meshzlength) (CallFunction|GetMeshLengths (Variables|Default|GetStaticMesh) (Variables|Default|GetAxisToScaleBy) false false false))
      (bind _output_get (Variables|Default|SetMeshLengthX _meshxlength))
      (bind _output_get_2 (Variables|Default|SetMeshLengthY _meshylength))
      (bind _output_get_3 (Variables|Default|SetMeshLengthZ _meshzlength)))
    (:then_2
      (bind _vectordistancesmadepositive (CallFunction|EnsureMakeVectorLengthPositive (Variables|Default|GetLastInstanceEnd)))
      (bind _output_get_4 (Variables|Default|SetDistanceToEndX (.x _vectordistancesmadepositive)))
      (bind _output_get_5 (Variables|Default|SetDistanceToEndY (.y _vectordistancesmadepositive)))
      (bind _output_get_6 (Variables|Default|SetDistanceToEndZ (.z _vectordistancesmadepositive))))
    (:then_3
      (bind (_scaletomatchend _instancecountx _instancecounty _instancecountz) (CallFunction|CalculateInstanceCountsandMeshScales (Math|Vector|MakeVector _output_get_4 _output_get_5 _output_get_6) (Math|Vector|MakeVector _output_get _output_get_2 _output_get_3)))
      (Variables|Default|SetScaleToMatchEndX (.x _scaletomatchend))
      (Variables|Default|SetScaleToMatchEndY (.y _scaletomatchend))
      (Variables|Default|SetScaleToMatchEndZ (.z _scaletomatchend))
      (Variables|Default|SetInstanceCount_X _instancecountx)
      (Variables|Default|SetInstanceCount_Y _instancecounty)
      (Variables|Default|SetInstanceCount_Z _instancecountz))
    (:then_4
      (if (Variables|Default|GetScaleToMatchEnd?)
        (for _index (range 0 (- (Variables|Default|GetInstanceCount_X) 1))
          (Components|InstancedStaticMesh|AddInstance (Variables|Default|GetInstanceGroupFloor) (Math|Transform|MakeTransform (Math|Vector|MakeVector (* (* (+ (Variables|Default|GetMeshLengthX) (.x (Variables|Default|GetCorrectionLength))) _index) (Variables|Default|GetScaleToMatchEndX)) 0.0 0.0) (Variables|Default|GetCorrectionRotation) (Math|Vector|MakeVector (Variables|Default|GetScaleToMatchEndX) (Variables|Default|GetScaleToMatchEndY) 1.0)) false)
          (for _index_2 (range 0 (- (Variables|Default|GetInstanceCount_Y) 2))
            (Components|InstancedStaticMesh|AddInstance (Variables|Default|GetInstanceGroupFloor) (Math|Transform|MakeTransform (Math|Vector|MakeVector (* (Variables|Default|GetScaleToMatchEndX) (* (+ (Variables|Default|GetMeshLengthX) (.x _correctionlength)) _index)) (* (Variables|Default|GetScaleToMatchEndY) (* (+ (Variables|Default|GetMeshLengthY) (.y _correctionlength)) (+ _index_2 1))) 0.0) (Variables|Default|GetCorrectionRotation) (Math|Vector|MakeVector (Variables|Default|GetScaleToMatchEndX) (Variables|Default|GetScaleToMatchEndY) 1.0)) false)))
        (else
          (CallFunction|CreateInstancebyManualCount))))))

(fn CreateInstancebyManualCount
  (bind _correctionlength (Variables|Default|GetCorrectionLength))
  (for _index (range 0 (- (Variables|Default|GetManual_InstanceCountX) 1))
    (Components|InstancedStaticMesh|AddInstance (Variables|Default|GetInstanceGroupFloor) (Math|Transform|MakeTransform (Math|Vector|MakeVector (* (+ (Variables|Default|GetMeshLengthX) (.x (Variables|Default|GetCorrectionLength))) _index) 0.0 0.0) (Variables|Default|GetCorrectionRotation)) false)
    (for _index_2 (range 0 (- (Variables|Default|GetManual_InstanceCountY) 2))
      (Components|InstancedStaticMesh|AddInstance (Variables|Default|GetInstanceGroupFloor) (Math|Transform|MakeTransform (Math|Vector|MakeVector (* (+ (Variables|Default|GetMeshLengthX) (.x _correctionlength)) _index) (* (+ (Variables|Default|GetMeshLengthY) (.y _correctionlength)) (+ _index_2 1)) 0.0) (Variables|Default|GetCorrectionRotation)) false))))