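; Level-art tool actor that builds a modular wall grid from a chosen mesh as hierarchical instanced static meshes.
; The construction script measures the mesh and the LastInstanceEnd vector, then derives instance counts and scales.
; It either tiles scaled modules along X or Y and up Z to match that end, or uses manual counts, with correction offsets and rotation.
; CreateInstanceAndScaleToMatchEnd is never called here.
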(event EventBeginPlay)

(event Collision|EventActorBeginOverlap
  (params (OtherActor :type Actor%20Object%20Reference)))

(event EventTick
  (params (DeltaSeconds :type Float%20%28single-precision%29)))

(fn ConstructionScript
  (Utilities|FlowControl|Sequence
    (:then_0
      ;[1 1 1] Allowing the user to set the mesh
      (CallFunction|InstantiateSingleHierarchicalInstancedStaticMesh (Variables|Default|GetInstanceGroupWall) (Variables|Default|GetMeshModuleWall)))
    (:then_1
      (bind (_meshxlength _meshylength _meshzlength) (CallFunction|GetMeshLengths (Variables|Default|GetMeshModuleWall) (Variables|Default|GetAxisToScaleBy) false false false))
      (bind _output_get (Variables|Default|SetMeshLengthX _meshxlength))
      (bind _output_get_2 (Variables|Default|SetMeshLengthY _meshylength))
      (bind _output_get_3 (Variables|Default|SetMeshLengthZ _meshzlength)))
    (:then_2
      (bind _vectordistancesmadepositive (CallFunction|EnsureMakeVectorLengthPositive (Variables|Default|GetLastInstanceEnd)))
      (bind _output_get_4 (Variables|Default|SetDistanceToEndX (.x _vectordistancesmadepositive)))
      (bind _output_get_5 (Variables|Default|SetDistanceToEndY (.y _vectordistancesmadepositive)))
      (bind _output_get_6 (Variables|Default|SetDistanceToEndZ (.z _vectordistancesmadepositive))))
    (:then_3
      (bind (_scaletomatchend _instancecountx _instancecounty _instancecountz) (CallFunction|CalculateInstanceCountsandMeshScales (Math|Vector|MakeVector _output_get_4 _output_get_5 _output_get_6) (Math|Vector|MakeVector _output_get _output_get_2 _output_get_3)))
      (Variables|Default|SetScaleToMatchEndX (.x _scaletomatchend))
      (Variables|Default|SetScaleToMatchEndY (.y _scaletomatchend))
      (Variables|Default|SetScaleToMatchEndZ (.z _scaletomatchend))
      (Variables|Default|SetInstanceCount_X _instancecountx)
      (Variables|Default|SetInstanceCount_Y _instancecounty)
      (Variables|Default|SetInstanceCount_Z _instancecountz))
    (:then_4
      (if (Variables|Default|GetScaleToMatchEnd?)
        ;[1 1 1] Checks if we are scaling by the x or y in the first slot
        (if (Utilities|Enum|Equal(Enum) (Utilities|Array|Get(acopy) (Variables|Default|GetAxisToScaleBy)) "NewEnumerator0")
          (CallFunction|CreateInstancebyUsingXZAxis)
          (else
            (CallFunction|CreateInstancebyUsingYZAxis)))
        (else
          (CallFunction|CreateInstancebyManualCount))))))

(fn CreateInstanceandScaletoMatchEnd
  (for _index (range 0 (- (Variables|Default|GetInstanceCount_X) 1))
    (Components|InstancedStaticMesh|AddInstance (Variables|Default|GetInstanceGroupWall) (Math|Transform|MakeTransform (Math|Vector|MakeVector (* (* (Variables|Default|GetMeshLengthX) _index) (Variables|Default|GetScaleToMatchEndX)) 0.0 0.0) "0, 0, 0" (Math|Vector|MakeVector (* 0.0 (Variables|Default|GetScaleToMatchEndX)) 0.0 0.0)) false)))

(fn CreateInstancebyManualCount
  (bind _correctionlengths (Variables|Default|GetCorrectionLengths))
  (bind _correctionlengths_2 (Variables|Default|GetCorrectionLengths))
  (for _index (range 0 (- (Variables|Default|GetMaunual_InstanceCount_Width) 1))
    (Components|InstancedStaticMesh|AddInstance (Variables|Default|GetInstanceGroupWall) (Math|Transform|MakeTransform (Math|Vector|MakeVector (* (+ (Variables|Default|GetMeshLengthX) (.x _correctionlengths_2)) _index) (* (+ (Variables|Default|GetMeshLengthY) (.y _correctionlengths_2)) _index) 0.0) (Variables|Default|GetCorrectionRotation)) false)
    (for _index_2 (range 0 (- (Variables|Default|GetManual_InstanceCount_Height) 2))
      (Components|InstancedStaticMesh|AddInstance (Variables|Default|GetInstanceGroupWall) (Math|Transform|MakeTransform (Math|Vector|MakeVector (* (+ (.x _correctionlengths) (Variables|Default|GetMeshLengthX)) _index) (* (+ (Variables|Default|GetMeshLengthY) (.y _correctionlengths)) _index) (* (+ (Variables|Default|GetMeshLengthZ) (.z _correctionlengths)) (+ _index_2 1))) (Variables|Default|GetCorrectionRotation)) false))))

(fn CreateInstancebyUsingXZAxis
  (bind _correctionlengths (Variables|Default|GetCorrectionLengths))
  ;[1 1 1] Using X axis
  (for _index (range 0 (- (Variables|Default|GetInstanceCount_X) 1))
    (Components|InstancedStaticMesh|AddInstance (Variables|Default|GetInstanceGroupWall) (Math|Transform|MakeTransform (Math|Vector|MakeVector (* (Variables|Default|GetScaleToMatchEndX) (* (+ (Variables|Default|GetMeshLengthX) (.x (Variables|Default|GetCorrectionLengths))) _index)) 0.0 0.0) (Variables|Default|GetCorrectionRotation) (Math|Vector|MakeVector (Variables|Default|GetScaleToMatchEndX) 1.0 (Variables|Default|GetScaleToMatchEndZ))) false)
    (for _index_2 (range 0 (- (Variables|Default|GetInstanceCount_Z) 2))
      (Components|InstancedStaticMesh|AddInstance (Variables|Default|GetInstanceGroupWall) (Math|Transform|MakeTransform (Math|Vector|MakeVector (* (Variables|Default|GetScaleToMatchEndX) (* (+ (Variables|Default|GetMeshLengthX) (.x _correctionlengths)) _index)) 0.0 (* (Variables|Default|GetScaleToMatchEndZ) (* (+ (Variables|Default|GetMeshLengthZ) (.z _correctionlengths)) (+ _index_2 1)))) (Variables|Default|GetCorrectionRotation) (Math|Vector|MakeVector (Variables|Default|GetScaleToMatchEndX) 1.0 (Variables|Default|GetScaleToMatchEndZ))) false))))

(fn CreateInstancebyUsingYZAxis
  (bind _correctionlengths (Variables|Default|GetCorrectionLengths))
  ;[1 1 1] using y axis
  (for _index (range 0 (- (Variables|Default|GetInstanceCount_Y) 1))
    (Components|InstancedStaticMesh|AddInstance (Variables|Default|GetInstanceGroupWall) (Math|Transform|MakeTransform (Math|Vector|MakeVector 0.0 (* (Variables|Default|GetScaleToMatchEndY) (* (+ (Variables|Default|GetMeshLengthY) (.y (Variables|Default|GetCorrectionLengths))) _index)) 0.0) (Variables|Default|GetCorrectionRotation) (Math|Vector|MakeVector 1.0 (Variables|Default|GetScaleToMatchEndY) (Variables|Default|GetScaleToMatchEndZ))) false)
    (for _index_2 (range 0 (- (Variables|Default|GetInstanceCount_Z) 2))
      (Components|InstancedStaticMesh|AddInstance (Variables|Default|GetInstanceGroupWall) (Math|Transform|MakeTransform (Math|Vector|MakeVector 0.0 (* (Variables|Default|GetScaleToMatchEndY) (* (+ (Variables|Default|GetMeshLengthY) (.y _correctionlengths)) _index)) (* (Variables|Default|GetScaleToMatchEndZ) (* (+ (Variables|Default|GetMeshLengthZ) (.z _correctionlengths)) (+ _index_2 1)))) (Variables|Default|GetCorrectionRotation) (Math|Vector|MakeVector 1.0 (Variables|Default|GetScaleToMatchEndY) (Variables|Default|GetScaleToMatchEndZ))) false))))