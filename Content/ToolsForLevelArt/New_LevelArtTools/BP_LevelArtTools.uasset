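; BP_LevelArtTools is a set of level-art helper functions for filling distances with instanced static meshes.
; Setup functions assign meshes to single or arrayed ISM and HISM components, matching by index for HISM arrays and using the first mesh for ISM arrays.
; Sizing helpers derive optionally negated per-axis lengths from mesh bounds and clamp distances to at least one.
; Rounded distance-to-length ratios give instance counts, plus scales that stretch instances to fit exactly.
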(fn InstantiateArrayHierarchicalInstancedStaticMeshes
  (params (HierarchicalInstancedMesh :type Array%20of%20Hierarchical%20Instanced%20Static%20Mesh%20Component%20Object%20References) (StaticMesh :type Array%20of%20Static%20Mesh%20Object%20References))
  ;[1 1 1] Allowing the user to set the mesh
  (for (_array_element _array_index) HierarchicalInstancedMesh
    (Components|StaticMesh|SetStaticMesh _array_element (Utilities|Array|Get(acopy) StaticMesh _array_index))))

(fn InstantiateArrayInstancedStaticMeshes
  (params (InstancedMesh :type Array%20of%20Instanced%20Static%20Mesh%20Component%20Object%20References) (StaticMesh :type Array%20of%20Static%20Mesh%20Object%20References))
  ;[1 1 1] Allowing the user to set the mesh
  (for _array_element InstancedMesh
    (Components|StaticMesh|SetStaticMesh _array_element (Utilities|Array|Get(acopy) StaticMesh))))

(fn InstantiateSingleHierarchicalInstancedStaticMesh
  (params (InstancedMesh :type Hierarchical%20Instanced%20Static%20Mesh%20Component%20Object%20Reference) (StaticMesh :type Static%20Mesh%20Object%20Reference))
  ;[1 1 1] Allowing the user to set the mesh
  (Components|StaticMesh|SetStaticMesh InstancedMesh StaticMesh))

(fn InstantiateSingleInstancedStaticMesh
  (params (InstancedMesh :type Instanced%20Static%20Mesh%20Component%20Object%20Reference) (StaticMesh :type Static%20Mesh%20Object%20Reference))
  ;[1 1 1] Allowing the user to set the mesh
  (Components|StaticMesh|SetStaticMesh InstancedMesh StaticMesh))

(fn GetMeshLengths
  (params (StaticMesh :type Static%20Mesh%20Object%20Reference) (NewParam :type Array%20of%20E_AxisToUse%20Enums :default "NewEnumerator0") (NegateX :type Boolean) (NegateY :type Boolean) (NegateZ :type Boolean))
  (bind _returnvalue (StaticMesh|GetBounds StaticMesh))
  (bind (_x _y _z) (Math|Vector|BreakVector (.boxextent _returnvalue)))
  (for _array_element NewParam
    (switch Utilities|FlowControl|Switch|SwitchonE_AxisToUse _array_element
      (:NewEnumerator0
        (bind _output_get (LocalVariables|SetMeshLengthX (* _x 2.0)))
        (if NegateX
          (LocalVariables|SetMeshLengthX (* _output_get -1.0))))
      (:NewEnumerator1
        (bind _output_get_2 (LocalVariables|SetMeshLengthY (* _y 2.0)))
        (if NegateY
          (LocalVariables|SetMeshLengthY (* _output_get_2 -1.0))))
      (:NewEnumerator2
        (bind _output_get_3 (LocalVariables|SetMeshLengthZ (* _z 2.0)))
        (if NegateZ
          (LocalVariables|SetMeshLengthZ (* _output_get_3 -1.0))))))
  (return (LocalVariables|GetMeshLengthX) (LocalVariables|GetMeshLengthY) (LocalVariables|GetMeshLengthZ)))

(fn EnsureMakeVectorLengthPositive
  (params (VectorDistance :type Vector))
  (return (Math|Vector|MakeVector (Math|Float|Max(Float) (.x VectorDistance) 1.0) (Math|Float|Max(Float) (.y VectorDistance) 1.0) (Math|Float|Max(Float) (.z VectorDistance) 1.0))))

(fn CalculateInstanceCountsandMeshScales
  (params (DistanceToEnd :type Vector) (MeshLengths :type Vector))
  (bind _returnvalue (Math|Float|Absolute(Float) (.y MeshLengths)))
  (bind _returnvalue_2 (Math|Float|Absolute(Float) (.x MeshLengths)))
  (bind _returnvalue_3 (Math|Float|Absolute(Float) (.z MeshLengths)))
  (bind _returnvalue_4 (/ (.y DistanceToEnd) _returnvalue))
  (bind _returnvalue_5 (/ (.x DistanceToEnd) _returnvalue_2))
  (bind _returnvalue_6 (/ (.z DistanceToEnd) _returnvalue_3))
  (bind _returnvalue_7 (Math|Float|Round _returnvalue_5))
  (bind _returnvalue_8 (Math|Float|Round _returnvalue_6))
  (bind _returnvalue_9 (Math|Float|Round _returnvalue_4))
  (return (Math|Vector|MakeVector (/ _returnvalue_5 (Math|Conversions|ToFloat(Integer) _returnvalue_7)) (/ _returnvalue_4 (Math|Conversions|ToFloat(Integer) _returnvalue_9)) (/ _returnvalue_6 (Math|Conversions|ToFloat(Integer) _returnvalue_8))) _returnvalue_7 _returnvalue_9 _returnvalue_8))