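; BP_ModularWallAndPillar is a level art tool that builds a straight run of modular walls and connector pieces along local X.
; The construction script divides the X distance to LastInstanceEnd by the wall mesh's bounds length, rounding to a module count.
; Walls are stretched slightly along X to fit exactly.
; Both user-set meshes use instanced components, with an offset connector at each wall's origin and none added at the far end.
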(event EventBeginPlay)

(event Collision|EventActorBeginOverlap
  (params (OtherActor :type Actor%20Object%20Reference)))

(event EventTick
  (params (DeltaSeconds :type Float%20%28single-precision%29)))

(fn ConstructionScript
  (bind _connectortransform (Variables|Default|GetConnectorTransform))
  (bind _walltransform (Variables|Default|GetWallTransform))
  (Utilities|FlowControl|Sequence
    (:then_0
      ;[1 1 1] Allowing the user to set the mesh
      (Components|StaticMesh|SetStaticMesh (Variables|Default|GetInstanceGroupWall) (Variables|Default|GetMeshModuleWall))
      (Components|StaticMesh|SetStaticMesh (Variables|Default|GetInstanceGroupConnector) (Variables|Default|GetMeshModuleConnector)))
    (:then_1
      (LocalVariables|SetMeshLength (* (.X (Math|Vector|BreakVector (.boxextent (StaticMesh|GetBounds (Variables|Default|GetMeshModuleWall))))) 2.0)))
    (:then_2
      (LocalVariables|SetDistanceToEnd (Math|Float|Max(Float) (.x (Variables|Default|GetLastInstanceEnd)) 1.0)))
    (:then_3
      (Variables|Default|SetInstanceCount (Math|Float|Round (/ (LocalVariables|GetDistanceToEnd) (LocalVariables|GetMeshLength))))
      (LocalVariables|SetScaleToMatchEnd (/ (/ (LocalVariables|GetDistanceToEnd) (LocalVariables|GetMeshLength)) (Math|Conversions|ToFloat(Integer) (Math|Float|Round (/ (LocalVariables|GetDistanceToEnd) (LocalVariables|GetMeshLength)))))))
    (:then_4
      (for _index (range 0 (- (Variables|Default|GetInstanceCount) 1))
        (Components|InstancedStaticMesh|AddInstance (Variables|Default|GetInstanceGroupWall) (Math|Transform|MakeTransform (Math|Vector|MakeVector (* (* (LocalVariables|GetMeshLength) _index) (LocalVariables|GetScaleToMatchEnd)) 0.0 0.0) "0, 0, 0" (Math|Vector|MakeVector (* (.x (.scale _walltransform)) (LocalVariables|GetScaleToMatchEnd)) (.y (.scale _walltransform)) (.z (.scale _walltransform)))) false)
        (Components|InstancedStaticMesh|AddInstance (Variables|Default|GetInstanceGroupConnector) (Math|Transform|MakeTransform (+ (.Location (Math|Transform|BreakTransform (Math|Transform|MakeTransform (Math|Vector|MakeVector (* (* (LocalVariables|GetMeshLength) _index) (LocalVariables|GetScaleToMatchEnd)) 0.0 0.0) "0, 0, 0" (Math|Vector|MakeVector (* (.x (.scale _walltransform)) (LocalVariables|GetScaleToMatchEnd)) (.y (.scale _walltransform)) (.z (.scale _walltransform)))))) (.location _connectortransform)) "0, 0, 0" (.scale _connectortransform)) false)))))