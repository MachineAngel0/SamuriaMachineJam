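; BP_Door is a door actor that slides its static mesh vertically when StartDoorMovement is called.
; The movement first resets the mesh to its relative origin, a testing measure that keeps repeated calls from stacking height.
; MoveComponentTo then eases the mesh to the Z of DoorMoveToLocation over DoorOpenSpeed, which serves as a duration, keeping its rotation.
; Nothing in the graph triggers the movement or closes the door.
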(event Custom|ResetDoorLocation
  ;[0.15 0.15 0.15 0.5] just reset its for testing purposes
  (Transformation|SetRelativeLocation (Variables|Default|GetStaticMesh) "0, 0, 0" false false))

(event Custom|StartDoorMovement
  ;[1 1 1] putting this here so the door doesn't infinite keep going up everytime this function is called
  (CallFunction|ResetDoorLocation)
  (Components|MoveComponentTo (Variables|Default|GetStaticMesh) (Math|Vector|MakeVector 0.0 0.0 (.z (Variables|Default|GetDoorMoveToLocation))) (Variables|/Script/Engine.SceneComponent|GetRelativeRotation (Variables|Default|GetStaticMesh)) true true (Variables|Default|GetDoorOpenSpeed) false))

(event EventBeginPlay)

(event Collision|EventActorBeginOverlap
  (params (OtherActor :type Actor%20Object%20Reference)))

(event EventTick
  (params (DeltaSeconds :type Float%20%28single-precision%29)))

(fn ConstructionScript)