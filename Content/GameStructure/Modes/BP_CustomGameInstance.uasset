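; BP_CustomGameInstance is a game instance that manages a single BP_CustomSaveGame in a named save slot.
; It exposes events to create, save, load and delete that save, keeping the active object in SaveGameFile.
; Loading creates and saves a new file when none exists, and reports a failed cast with a debug print.
; Saving and successful loading call GameSaved and GameLoaded with the save object, letting other systems react.
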(event Custom|CreateSaveGame
  (bind _returnvalue (SaveGame|CreateSaveGameObject "/Game/GameStructure/Modes/BP_CustomSaveGame.BP_CustomSaveGame_C"))
  (Variables|Default|SetSaveGameFile _returnvalue)
  (CallFunction|SaveGame))

(event Custom|LoadGame
  (bind _returnvalue (SaveGame|DoesSaveGameExist (Variables|Default|GetSaveSlotName)))
  (if _returnvalue
    (bind _returnvalue_2 (SaveGame|LoadGamefromSlot (Variables|Default|GetSaveSlotName)))
    (bind _asbp_custom_save_game (Utilities|Casting|CastToBP_CustomSaveGame _returnvalue_2)
      (:then
        (Variables|Default|SetSaveGameFile _asbp_custom_save_game)
        (Default|CallGameLoaded (Variables|Default|GetSaveGameFile)))
      (:CastFailed
        (Development|PrintString "Cast To Custom Save Game Failed")))
    (else
      (CallFunction|CreateSaveGame)
      (Default|CallGameLoaded (Variables|Default|GetSaveGameFile)))))

(event Custom|SaveGame
  (SaveGame|SaveGametoSlot (Variables|Default|GetSaveGameFile) (Variables|Default|GetSaveSlotName))
  (Default|CallGameSaved (Variables|Default|GetSaveGameFile)))

(event Custom|DeleteSave
  (bind _returnvalue (SaveGame|DoesSaveGameExist (Variables|Default|GetSaveSlotName)))
  (if _returnvalue
    (SaveGame|DeleteGameinSlot (Variables|Default|GetSaveSlotName))))