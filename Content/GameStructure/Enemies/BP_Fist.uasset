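; BP_Fist is an enemy Blueprint that performs Fist and Charge attacks when given an AI action.
; PerformAIAction switches on the action type, prints the attack name, signals a new enemy state and plays that attack's montage on the mesh, using sword-and-shield slash and Shadow Knight charge animations.
; When the montage completes, it signals a second state; interruption is not handled.
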(event EventBeginPlay)

(event Collision|EventActorBeginOverlap
  (params (OtherActor :type Actor%20Object%20Reference)))

(event EventTick
  (params (DeltaSeconds :type Float%20%28single-precision%29)))

(event EventPerformAIAction
  (params (EnemyAIActionType :type E_EnemyAIActionType%20Enum :default "NewEnumerator0"))
  (switch Utilities|FlowControl|Switch|SwitchonE_EnemyAIActionType EnemyAIActionType
    (:NewEnumerator0
      (Development|PrintString "FistAttack")
      (CallFunction|SignalNewEnemyState "NewEnumerator6")
      (Animation|Montage|PlayMontage (Variables|Character|GetMesh) "/Game/AssetPacks/ShadowKnight/Animations/SKSwordAndShieldSlashCombo1_Montage.SKSwordAndShieldSlashCombo1_Montage"
        (:OnCompleted
          (CallFunction|SignalNewEnemyState "NewEnumerator4"))))
    (:NewEnumerator1
      (Development|PrintString "ChargeAttack")
      (CallFunction|SignalNewEnemyState "NewEnumerator6")
      (Animation|Montage|PlayMontage (Variables|Character|GetMesh) "/Game/AssetPacks/ShadowKnight/Animations/AM_ShadowKnight_ChargeAttack.AM_ShadowKnight_ChargeAttack"
        (:OnCompleted
          (CallFunction|SignalNewEnemyState "NewEnumerator4"))))))

(fn ConstructionScript)