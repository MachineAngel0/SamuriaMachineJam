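; Base enemy character that takes damage, shows a health widget and can drop a key on death.
; BeginPlay binds the WB_HealthUI widget to the health component and registers for its death signal, while DoDamage feeds that component and plays a hurt sound.
; Death runs once, ragdolling the mesh, detaching the controller, hiding the widget and optionally spawning a key pickup.
; Enemy state changes are relayed through an event dispatcher.
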(event Custom|OnDeathEvent
  (bind _mesh (Variables|Character|GetMesh))
  (Utilities|FlowControl|DoOnce false
    (:Completed
      (Collision|SetCollisionResponsetoAllChannels _mesh "ECR_Block")
      (Collision|SetCollisionEnabled _mesh "PhysicsOnly")
      (Collision|SetCollisionEnabled (Variables|Collision|GetCapsuleComponent) "NoCollision")
      (Physics|SetSimulatePhysics _mesh true)
      ;[1 1 1] Destroys the ai controller
      (Class|Pawn|DetachfromControllerPendingDestroy)
      (Development|SetHiddeninGame (Variables|Default|GetWidget) true false)
      (if (Variables|Default|GetDropAKey?)
        (Game|SpawnActorfromClass "/Game/GameStructure/Player/BP_KeyPickUp.BP_KeyPickUp_C" (Transformation|GetWorldTransform (Variables|Default|GetKeyDropLocation)) "Undefined" "MultiplyWithRoot" 0 (Variables|Default|GetKeyToDrop) 0)))))

(event Custom|SignalNewEnemyState
  (params (NewEnemyState :type E_EnemyState%20Enum :default "NewEnumerator0"))
  (Default|CallOnEnemyStateChange NewEnemyState))

(event EventBeginPlay
  (bind _widget (Variables|Default|GetWidget))
  (bind _bpc_healthcomponent (Variables|Default|GetBPC_HealthComponent))
  (bind _returnvalue (UserInterface|GetWidget _widget))
  (if (Class|GameplayStatics|ObjectIsA _returnvalue "/Game/GameStructure/UI/WB_HealthUI.WB_HealthUI_C")
    (bind _aswb_health_ui (Utilities|Casting|CastToWB_HealthUI _returnvalue))
    ;[1 1 1] create signal bindings for the health
    (Default|Initialize _aswb_health_ui (Variables|Default|GetBPC_HealthComponent))
    ;[1 1 1] signal the health to update, so that the UI is up to date
    (Default|SignalHealthChange _bpc_healthcomponent)
    (EventDispatchers|AssignOnDeath _bpc_healthcomponent (EventDispatchers|CreateEvent :!event Custom|OnDeathEvent))))

(event Collision|EventActorBeginOverlap
  (params (OtherActor :type Actor%20Object%20Reference)))

(event EventTick
  (params (DeltaSeconds :type Float%20%28single-precision%29)))

(fn ConstructionScript)

(fn DoDamage
  (params (DamagingActor :type Actor%20Object%20Reference) (DamageAmount :type Float%20%28double-precision%29))
  (Default|TakeDamage (Variables|Default|GetBPC_HealthComponent) DamageAmount)
  (Audio|PlaySound2D (Variables|Default|GetDamagedSound) 1.0 1.0 0.0 0 0)
  (return true))