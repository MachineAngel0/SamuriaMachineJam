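; BPC_HealthComponent is a component that tracks health and death state for its owner.
; TakeDamage subtracts damage from current health without clamping, broadcasts the new health as a fraction of max health, then checks for death.
; At zero or below it sets IsDead and fires the death dispatcher, with no guard against firing again on later hits.
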(event Custom|TakeDamage
  (params (DamageAmount :type Float%20%28double-precision%29))
  (Variables|Default|SetCurrentHealth (- (Variables|Default|GetCurrentHealth) DamageAmount))
  (CallFunction|SignalHealthChange)
  (CallFunction|CheckifDead))

(event Custom|SignalHealthChange
  (Default|CallOnHealthChange (CallFunction|GetHealthPercent)))

(event Custom|Check%20If%20Dead
  (bind _currenthealth (Variables|Default|GetCurrentHealth))
  (bind _returnvalue (<= _currenthealth 0.0))
  (if _returnvalue
    (Variables|Default|SetIsDead _returnvalue)
    (Default|CallOnDeath)))

(event EventBeginPlay)

(event EventTick
  (params (DeltaSeconds :type Float%20%28single-precision%29)))

(fn GetHealthPercent
  (return (/ (Variables|Default|GetCurrentHealth) (Variables|Default|GetMaxHealth))))