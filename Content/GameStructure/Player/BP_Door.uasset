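; BP_Door is an interactable keyed door that the player opens by holding the matching key.
; Interact rejects non-player actors, then checks the BP_CEPlayerCharacter's KeysArray for KeyToCheckFor, printing a message if the key is missing or the door is already open.
; A successful check sets IsDoorOpen, resets the mesh position, plays a 2D sound and eases the mesh vertically to DoorMoveToLocation's Z via MoveComponentTo.
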(event Custom|ResetDoorLocation
  ;[0.15 0.15 0.15 0.5] just reset its for testing purposes
  (Transformation|SetRelativeLocation (Variables|Default|GetStaticMesh) "0, 0, 0" false false))

(event Custom|StartDoorMovement
  (Variables|Default|SetIsDoorOpen? true)
  ;[1 1 1] putting this here so the door doesn't infinitly keep going up everytime this function is called
  (CallFunction|ResetDoorLocation)
  ;[1 1 1] sound goes on for a bit too long
  (Audio|PlaySound2D (Variables|Default|GetDoorOpenSound) 1.0 1.0 0.0 0 0)
  (Components|MoveComponentTo (Variables|Default|GetStaticMesh) (Math|Vector|MakeVector 0.0 0.0 (.z (Variables|Default|GetDoorMoveToLocation))) (Variables|/Script/Engine.SceneComponent|GetRelativeRotation (Variables|Default|GetStaticMesh)) true true (Variables|Default|GetDoorOpenSpeed) false))

(event EventBeginPlay)

(event Collision|EventActorBeginOverlap
  (params (OtherActor :type Actor%20Object%20Reference)))

(event EventTick
  (params (DeltaSeconds :type Float%20%28single-precision%29)))

(fn ConstructionScript)

(fn Interact
  (params (RequestingActor :type Actor%20Object%20Reference))
  (if (Variables|Default|GetIsDoorOpen?)
    (Development|PrintString "door is already open")
    (elif (Class|GameplayStatics|ObjectIsA RequestingActor "/Game/GameStructure/Player/BP_CEPlayerCharacter.BP_CEPlayerCharacter_C")
      (bind _asbp_ceplayer_character (Utilities|Casting|CastToBP_CEPlayerCharacter RequestingActor))
      (if (Utilities|Array|ContainsItem (Variables|/Game/GameStructure/Player/BP_CEPlayerCharacter.BP_CEPlayerCharacter_C|GetKeysArray _asbp_ceplayer_character) (Variables|Default|GetKeyToCheckFor))
        (CallFunction|StartDoorMovement)
        (return true)
        (else
          (Development|PrintString "Do not have the right key to open door")
          (return false)))
      (else
        (return false)))))